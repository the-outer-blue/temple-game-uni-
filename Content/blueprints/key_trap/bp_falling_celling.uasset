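; Falling ceiling trap Blueprint that extends spikes, then lowers the ceiling to kill whatever it catches.
; The smush event plays a timeline that slides the Box down, pauses briefly, then arms CanKill and starts the Movement timeline.
; Movement lowers the Plane at a play rate scaled by TimeToFall.
; Once armed, any actor that begins overlapping the Box receives DeathMessage.
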(event `smush`
  ;[0.15 0 0.0231 0.5] have spikes appear
  (bind (_direction _movement) (`Timeline|spikes_appear` :!via `PlayFromStart`)
    (:`Update`
      (`SceneComponent.K2_SetRelativeLocation` (`self.Box`) (`KismetMathLibrary.VLerp` (0.0 0.0 45.0) (0.0 0.0 -30.0) _movement) false false))
    (:`Finished`
      (`KismetSystemLibrary.Delay` 0.3)
      ;[0 0.15 0.1234 0.5] move ceeling down
      (set `self.can kill` true)
      (`TimelineComponent.SetPlayRate` (`self.movement`) (/ 5.0 (`self.time to fall`)))
      (bind (_direction_2 _movement_2) (`Timeline|movement` :!via `PlayFromStart`)
        (:`Update`
          (`SceneComponent.K2_SetRelativeLocation` (`self.Plane`) (`KismetMathLibrary.VLerp` (0.0 0.0 400.0) (0.0 0.0 0.0) _movement_2) false false))))))

(event `self.Box.OnComponentBeginOverlap`
  (params (OverlappedComponent :type "PrimitiveComponent Object Reference") (OtherActor :type "Actor Object Reference") (OtherComp :type "PrimitiveComponent Object Reference") (OtherBodyIndex :type Integer) (bFromSweep :type Boolean) (SweepResult :type "HitResult Structure (by ref)"))
  ;[0.01672 0.15 0 0.5] kill player
  (if (`self.can kill`)
    (message `/Game/blueprints/bp_player_interface.death` OtherActor)))

(fn `UserConstructionScript`)