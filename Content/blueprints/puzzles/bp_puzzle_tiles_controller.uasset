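; Puzzle controller Blueprint that opens a door when a set of tiles shows the correct code.
; The check_code event loops over the tile array and compares each tile's Code plus one against the matching SolveCode entry.
; Any mismatch clears IsSolved; if all match, it calls Open on the referenced Door.
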(event `check_code`
  ;[0 0.1365 0.15 0.5] check if code is correct
  (set `self.is solved` true)
  (for (_array_element _array_index) (`self.puzzle tles`)
    (if (not (== (+ (`/Game/blueprints/puzzles/bp_puzzle_tile.code` _array_element) 1) (`|GetArrayItem` (`self.solve code`) _array_index)))
      (set `self.is solved` false)))
  (if (`self.is solved`)
    (`/Game/blueprints/puzzles/BP_door.open` (`self.door`))))

(fn `UserConstructionScript`)