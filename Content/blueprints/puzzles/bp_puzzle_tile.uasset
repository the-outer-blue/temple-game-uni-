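; Puzzle tile Blueprint that cycles its code number each time it is interacted with and shows it through light colour.
; Interact increments Code, wraps it to zero past MaxOptions and sets the point light to the Colour array entry at that index.
; BeginPlay resizes the Colour array so it has an entry for every possible code.
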(event `self.ReceiveBeginPlay`
  ; ensure theres enough options in the array
  (`KismetArrayLibrary.Array_Resize` (`self.colour`) (+ (`self.max_options`) 1)))

(event `/Game/blueprints/bp_interact_interface.interact`
  (bind _code (`self.code`))
  ;[0.02241 0.15 0 0.5] increase code number
  (bind _result (`/Engine/EditorBlueprintResources/StandardMacros.IncrementInt` _code)
    (:`  `
      (if (not (<= _result (`self.max_options`)))
        (set `self.code` 0))
      (`LightComponent.SetLightColor` (`self.PointLight`) (`KismetMathLibrary.Conv_ColorToLinearColor` (`|GetArrayItem` (`self.colour`) _code)) true))))

(fn `UserConstructionScript`)