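; Lever actor for a tile puzzle that opens a door when the player sets the correct code.
; On Interact it compares each puzzle tile's Value plus one against the matching SolveCode entry, clearing IsSolved on any mismatch.
; If every tile matches, it calls Open on the referenced Door.
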(event `/Game/blueprints/bp_player_interface.interact`
  ;[0 0.1365 0.15 0.5] check if code is correct
  (set `self.Is solved` true)
  (for (_array_element _array_index) (`self.Puzzle Tiles`)
    (if (not (== (+ (`/Game/blueprints/tile_puzzle/bp_puzzle_tile.value` _array_element) 1) (`|GetArrayItem` (`self.solve code`) _array_index)))
      (set `self.Is solved` false)))
  ;[0 0.15 0.05531 0.5] open door if correct
  (if (`self.Is solved`)
    (`/Game/blueprints/tile_puzzle/BP_door.open` (`self.door`))))

(fn `UserConstructionScript`)