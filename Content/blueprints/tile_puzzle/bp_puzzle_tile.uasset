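; Puzzle tile actor that shows one of several symbols through a decal, forming one digit of a code puzzle.
; Each interaction increments its Value, wrapping to zero after three states, and swaps the decal material from the Symbols array.
; The construction script applies the symbol for the initial Value, so the starting state shows in the editor.
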(event `/Game/blueprints/bp_player_interface.interact`
  (bind _value (`self.value`))
  ;[0.02241 0.15 0 0.5] increase code number
  (`/Engine/EditorBlueprintResources/StandardMacros.IncrementInt` _value
    (:`  `
      (if (not (< _value 3))
        (set `self.value` 0))
      (`DecalComponent.SetDecalMaterial` (`self.Decal`) (`|GetArrayItem` (`self.symbols`) (`self.value`))))))

(fn `UserConstructionScript`
  (`DecalComponent.SetDecalMaterial` (`self.Decal`) (`|GetArrayItem` (`self.symbols`) (`self.value`))))