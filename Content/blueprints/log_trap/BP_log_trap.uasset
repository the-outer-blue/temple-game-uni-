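; Log trap that swings a collision Box toward an endpoint and kills what it overlaps while lethal.
; The swing event arms the trap and, gated by a DoOnce until finished, plays a timeline with separate Y and Z curves driving the Box's relative location.
; A timeline track also toggles CanKill, so overlaps send DeathMessage to the other actor only during lethal parts of the swing.
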(event `swing`
  (bind (_endpoint_x _endpoint_y _endpoint_z) (`KismetMathLibrary.BreakVector` (`self.endpoint`)))
  ;[0.15 0 0 0.5] swing the log
  (set `self.can kill` true)
  (`/Engine/EditorBlueprintResources/StandardMacros.DoOnce` false :!label _label
    (:`Completed`
      (bind (_direction __y_value _z_value _can_kill) (`Timeline|swing momentum` :!via `PlayFromStart`)
        (:`Update`
          (set `self.can kill` (== _can_kill 1.0))
          (`SceneComponent.K2_SetRelativeLocation` (`self.Box`) (`KismetMathLibrary.MakeVector` 0.0 (`KismetMathLibrary.Lerp` 0.0 _endpoint_y __y_value) (`KismetMathLibrary.Lerp` 0.0 _endpoint_z _z_value)) false false))
        (:`Finished`
          (goto _label :!via `Reset`))))))

(event `self.Box.OnComponentBeginOverlap`
  (params (OverlappedComponent :type "PrimitiveComponent Object Reference") (OtherActor :type "Actor Object Reference") (OtherComp :type "PrimitiveComponent Object Reference") (OtherBodyIndex :type Integer) (bFromSweep :type Boolean) (SweepResult :type "HitResult Structure (by ref)"))
  ;[0.15 0.1329 0.01405 0.5] kills player
  (if (`self.can kill`)
    (message `/Game/blueprints/bp_player_interface.death` OtherActor)))

(fn `UserConstructionScript`)