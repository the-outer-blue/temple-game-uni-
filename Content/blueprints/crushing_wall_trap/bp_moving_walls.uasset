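; Crushing wall trap actor that slides two walls inward to kill what is caught between them.
; A crush event arms the kill flag and plays a timeline that lerps both walls toward the center, mirroring the second by negating the first's position.
; Two box overlaps send DeathMessage to the overlapping actor once armed, and nothing in the graph disarms the trap.
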(event `crush`
  ;[0.007568 0.15 0 0.5] moves walls toward center
  (set `self.can kill` true)
  (bind (_direction _movement) (`Timeline|moving walls`)
    (:`Update`
      (bind _returnvalue (`KismetMathLibrary.VLerp` (200.0 0.0 0.0) (0.0 0.0 0.0) _movement))
      (`SceneComponent.K2_SetRelativeLocation` (`self.wall 1`) _returnvalue false false)
      (`SceneComponent.K2_SetRelativeLocation` (`self.wall 2`) (* _returnvalue -1.0) false false))))

(event `self.Box1.OnComponentBeginOverlap`
  (params (OverlappedComponent :type "PrimitiveComponent Object Reference") (OtherActor :type "Actor Object Reference") (OtherComp :type "PrimitiveComponent Object Reference") (OtherBodyIndex :type Integer) (bFromSweep :type Boolean) (SweepResult :type "HitResult Structure (by ref)"))
  ;[0.001801 0.03252 0.15 0.5] kill player when overlapped
  (`KismetSystemLibrary.PrintString` "Hello")
  (if (`self.can kill`)
    (message `/Game/blueprints/bp_player_interface.death` OtherActor)))

(event `self.Box.OnComponentBeginOverlap`
  (params (OverlappedComponent :type "PrimitiveComponent Object Reference") (OtherActor :type "Actor Object Reference") (OtherComp :type "PrimitiveComponent Object Reference") (OtherBodyIndex :type Integer) (bFromSweep :type Boolean) (SweepResult :type "HitResult Structure (by ref)"))
  ;[0.001801 0.03252 0.15 0.5] kill player when overlapped
  (`KismetSystemLibrary.PrintString` "Hello")
  (if (`self.can kill`)
    (message `/Game/blueprints/bp_player_interface.death` OtherActor)))

(fn `UserConstructionScript`)